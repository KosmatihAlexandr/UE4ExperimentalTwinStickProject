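; BP_EnamySpawner is an actor that periodically spawns BP_EnamyCharacter enemies at its location.
; From BeginPlay, a non-looping timer re-arms itself at a random interval after every Spawn attempt.
; A Box overlap keeps a list of player characters inside, and spawning is skipped while any are present or the world's enemy count exceeds a cap.
; Each new enemy appears slightly above the spawner and receives its default controller.
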(event `Spawn`
  (bind _outactors (`GameplayStatics.GetAllActorsOfClass` "/Game/Characters/Blueprints/NPC/BP_EnamyCharacter.BP_EnamyCharacter_C"))
  (if (not (or (> (`KismetArrayLibrary.Array_Length` (`self.OverlapingPlayers`)) 0) (> (`KismetArrayLibrary.Array_Length` _outactors) 10)))
    (bind _returnvalue (`|SpawnActorFromClass` "/Game/Characters/Blueprints/NPC/BP_EnamyCharacter.BP_EnamyCharacter_C" (`KismetMathLibrary.MakeTransform` (+ (`self.K2_GetActorLocation`) (0.0 0.0 100.0))) "Undefined" "OverrideRootScale" null null))
    (`Pawn.SpawnDefaultController` _returnvalue))
  (`KismetSystemLibrary.K2_SetTimerDelegate` (delegate `Spawn`) (`KismetMathLibrary.RandomFloatInRange` 5.0 30.0) :!label _label))

(event `self.ReceiveBeginPlay`
  (goto _label))

(event `self.Box.OnComponentBeginOverlap`
  (params (OverlappedComponent :type "PrimitiveComponent Object Reference") (OtherActor :type "Actor Object Reference") (OtherComp :type "PrimitiveComponent Object Reference") (OtherBodyIndex :type Integer) (bFromSweep :type Boolean) (SweepResult :type "HitResult Structure (by ref)"))
  (bind _asbp_player_character (cast `/Game/Characters/Blueprints/Player/BP_PlayerCharacter` OtherActor))
  (`KismetArrayLibrary.Array_AddUnique` (`self.OverlapingPlayers`) _asbp_player_character))

(event `self.Box.OnComponentEndOverlap`
  (params (OverlappedComponent :type "PrimitiveComponent Object Reference") (OtherActor :type "Actor Object Reference") (OtherComp :type "PrimitiveComponent Object Reference") (OtherBodyIndex :type Integer))
  (bind _asbp_player_character (cast `/Game/Characters/Blueprints/Player/BP_PlayerCharacter` OtherActor))
  (`KismetArrayLibrary.Array_RemoveItem` (`self.OverlapingPlayers`) _asbp_player_character))

(fn `UserConstructionScript`)