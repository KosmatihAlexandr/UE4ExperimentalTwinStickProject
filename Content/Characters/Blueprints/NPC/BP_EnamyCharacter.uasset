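; Enemy NPC character Blueprint that spawns armed and changes walk speed with its suspicion state.
; On BeginPlay, SimpleWeaponManager equips a random pistol, rifle or shotgun, and GetWeaponType reads from it, falling back to Pistol.
; Suspesious is a RepNotify variable whose handler calls UpdateWalkSpeed, selecting fast speed when suspicious and not aiming, otherwise normal.
; The construction script starts movement at normal walk speed.
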(event `self.ReceiveBeginPlay`
  (`SimpleWeaponManager.TakeWeapon` (`self.SimpleWeaponManager`) (select `int` (`KismetMathLibrary.RandomIntegerInRange` 0 2) :`0` "/Game/Weapons/BP_Pistol.BP_Pistol_C" :`1` "/Game/Weapons/BP_Rifle.BP_Rifle_C" :`2` "/Game/Weapons/BP_Shotgun.BP_Shotgun_C" :!type "BaseWeaponComponent Class Reference")))

(event `self.ReceiveTick`
  (params (DeltaSeconds :type "Float (single-precision)"))
  (`parent.ReceiveTick` DeltaSeconds))

(event `self.UpdateWalkSpeed`
  (set `CharacterMovementComponent.MaxWalkSpeed` (select `bool` (or (`self.Aiming`) (not (`self.Suspesious`))) :`false` (`self.FastWalkSpeed`) :`true` (`self.NormalWalkSpeed`)) (`self.CharacterMovement`)))

(fn `GetWeaponType`
  (returns (WeaponType :type "EWeaponType Enum"))
  (bind _simpleweaponmanager (`self.SimpleWeaponManager`))
  (`/Engine/EditorBlueprintResources/StandardMacros.IsValid` _simpleweaponmanager
    (:`Is Valid`
      (return (`WeaponManager.GetWeaponType` _simpleweaponmanager)))
    (:`Is Not Valid`
      (return "Pistol"))))

(fn `OnRep_Suspesious`
  (`self.UpdateWalkSpeed`))

(fn `SetSuspesious`
  (params (Suspecious :type Boolean))
  (set `self.Suspesious` Suspecious))

(fn `UserConstructionScript`
  (`parent.UserConstructionScript`)
  (set `CharacterMovementComponent.MaxWalkSpeed` (`self.NormalWalkSpeed`) (`self.CharacterMovement`)))