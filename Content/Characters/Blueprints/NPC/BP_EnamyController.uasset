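; AI controller for enemy NPCs that runs the patrol behavior tree and caches the possessed enemy character.
; Sight of an actor with a differing first tag sets the blackboard target and focus; losing it, or sensing other stimuli, records a suspicious point.
; A Tick-fed gate optionally turns the controller toward random yaws at a capped rate.
; Helper functions forward aiming, shooting, weapon range and suspicion to the character.
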(event `self.ReceiveBeginPlay`
  (`self.RunBehaviorTree` "/Game/Characters/Blueprints/NPC/BT_EnamyPatrol.BT_EnamyPatrol")
  (bind _asbp_enamy_character (cast `/Game/Characters/Blueprints/NPC/BP_EnamyCharacter` (`self.K2_GetPawn`)))
  (set `self.ControledPawn` _asbp_enamy_character))

(event `self.AIPerception.OnTargetPerceptionUpdated`
  (params (Actor :type "Actor Object Reference") (Stimulus :type "AIStimulus Structure"))
  (bind (_age _expirationage _strength _stimuluslocation _receiverlocation _tag _bsuccessfullysensed) (break `AIStimulus` Stimulus))
  (bind _returnvalue (`AIBlueprintHelperLibrary.GetBlackboard` null))
  (bind _targetkey (`self.TargetKey`))
  (bind _returnvalue_2 (`AIPerceptionSystem.GetSenseClassForStimulus` Stimulus))
  (if (== _returnvalue_2 "/Script/AIModule.AISense_Sight")
    (if (!= (`|GetArrayItem` (`Actor.Tags` Actor)) (`|GetArrayItem` (`Actor.Tags` (`self.ControledPawn`))))
      (if _bsuccessfullysensed
        (`BlackboardComponent.SetValueAsObject` _returnvalue _targetkey Actor)
        (`self.K2_SetFocus` Actor)
        (else
          (`BlackboardComponent.SetValueAsVector` _returnvalue (`self.SuspiciousPointKey`) (`self.K2_GetActorLocation` Actor))
          (`BlackboardComponent.ClearValue` _returnvalue _targetkey)
          (`self.K2_ClearFocus`))))
    (elif _bsuccessfullysensed
      (`BlackboardComponent.SetValueAsVector` (`AIBlueprintHelperLibrary.GetBlackboard` null) (`self.SuspiciousPointKey`) _stimuluslocation))))

(event `ActivateRandomRotation`
  (params (Active :type Boolean))
  (bind (_returnvalue_roll _returnvalue_pitch _returnvalue_yaw) (`KismetMathLibrary.BreakRotator` (`self.K2_GetActorRotation`)))
  (bind _randdirection (`self.RandDirection`))
  (bind (_returnvalue_roll_2 _returnvalue_pitch_2 _returnvalue_yaw_2) (`KismetMathLibrary.BreakRotator` (`KismetMathLibrary.NormalizedDeltaRotator` (`KismetMathLibrary.MakeRotator` 0.0 0.0 _randdirection) (`KismetMathLibrary.MakeRotator` 0.0 0.0 _returnvalue_yaw))))
  (if Active
    (set `self.RandDirection` (`KismetMathLibrary.RandomFloatInRange` -180.0 180.0))
    (goto _label :!via `Open`)
    (else
      (goto _label :!via `Close`))))

(event `self.ReceiveTick`
  (params (DeltaSeconds :type "Float (single-precision)"))
  (bind (_returnvalue_roll _returnvalue_pitch _returnvalue_yaw) (`KismetMathLibrary.BreakRotator` (`self.K2_GetActorRotation`)))
  (bind _returnvalue (* DeltaSeconds 45.0))
  (bind _randdirection (`self.RandDirection`))
  (bind (_returnvalue_roll_2 _returnvalue_pitch_2 _returnvalue_yaw_2) (`KismetMathLibrary.BreakRotator` (`KismetMathLibrary.NormalizedDeltaRotator` (`KismetMathLibrary.MakeRotator` 0.0 0.0 _randdirection) (`KismetMathLibrary.MakeRotator` 0.0 0.0 _returnvalue_yaw))))
  (`/Engine/EditorBlueprintResources/StandardMacros.Gate` true :!label _label
    (:`Exit`
      (bind _result (`/Engine/EditorBlueprintResources/StandardMacros.NegateFloat` _returnvalue)
        (:`  `
          (`self.K2_AddActorWorldRotation` (`KismetMathLibrary.MakeRotator` 0.0 0.0 (`KismetMathLibrary.ClampAngle` _returnvalue_yaw_2 _result _returnvalue)))
          (if (== _returnvalue_yaw _randdirection)
            (set `self.RandDirection` (`KismetMathLibrary.RandomFloatInRange` -180.0 180.0))))))))

(fn `GetWeaponRange`
  (returns (Distance :type "Float (double-precision)"))
  (return (`WeaponManager.GetWeaponFiringRange` (`/Game/Characters/Blueprints/NPC/BP_EnamyCharacter.SimpleWeaponManager` (`self.ControledPawn`)))))

(fn `SetAimToEnamy`
  (params (Aim :type Boolean))
  (set `/Game/Characters/AnimStarterPack/Ue4ASP_Character.Aiming` Aim (`self.ControledPawn`)))

(fn `SetSuspection`
  (params (Suspicious :type Boolean))
  (`/Game/Characters/Blueprints/NPC/BP_EnamyCharacter.SetSuspesious` (`self.ControledPawn`) Suspicious))

(fn `StartShooting`
  (params (start :type Boolean))
  (bind _simpleweaponmanager (`/Game/Characters/Blueprints/NPC/BP_EnamyCharacter.SimpleWeaponManager` (`self.ControledPawn`)))
  (if start
    (`WeaponManager.StartShooting` _simpleweaponmanager)
    (else
      (`WeaponManager.StopShooting` _simpleweaponmanager))))

(fn `UserConstructionScript`)