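; Behavior Tree decorator for NPCs that passes while the controlled pawn is moving or a countdown is still running.
; The condition check casts the owner to a Controller and tests whether its pawn's velocity is at least a small threshold, or DeltaTime is above zero.
; Tick drains DeltaTime by the frame's delta seconds, and neither graph resets it.
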(event `self.ReceiveTick`
  (params (OwnerActor :type "Actor Object Reference") (DeltaSeconds :type "Float (single-precision)"))
  (set `self.DeltaTime` (- (`self.DeltaTime`) DeltaSeconds)))

(fn `PerformConditionCheck`
  (params (OwnerActor :type "Actor Object Reference"))
  (returns (ReturnValue :type Boolean))
  (bind _ascontroller (cast `Controller` OwnerActor))
  (return (or (>= (`KismetMathLibrary.VSize` (`Actor.GetVelocity` (`Controller.K2_GetPawn` _ascontroller))) 0.1) (> (`self.DeltaTime`) 0.0))))